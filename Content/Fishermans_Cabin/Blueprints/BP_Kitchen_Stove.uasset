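; BP_Kitchen_Stove is a configurable kitchen stove prop for the Fisherman's Cabin environment, with no active runtime logic.
; Its Construction Script rotates the door and five dial meshes from angle variables and toggles the cable mesh's visibility.
; It also creates a dynamic material instance on one stove mesh to set the oven's emissive strength.
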(event EventBeginPlay)

(event Collision|EventActorBeginOverlap
  (params (OtherActor :type Actor%20Object%20Reference)))

(event EventTick
  (params (DeltaSeconds :type Float%20%28single-precision%29)))

(fn ConstructionScript
  (Transformation|AddRelativeRotation (Variables|Default|GetKitchen_Stove_02) (Math|Rotator|MakeRotator (* (Variables|Stove|GetDoor%20Open%20Angle) -1.0) 0.0 0.0) false false)
  (Transformation|AddLocalRotation (Variables|Default|GetKitchen_Stove_06) (Math|Rotator|MakeRotator 0.0 (Variables|Stove|GetDial%2001%20Rotation) 0.0) false false)
  (Transformation|AddLocalRotation (Variables|Default|GetKitchen_Stove_07) (Math|Rotator|MakeRotator 0.0 (Variables|Stove|GetDial%2002%20Rotation) 0.0) false false)
  (Transformation|AddLocalRotation (Variables|Default|GetKitchen_Stove_08) (Math|Rotator|MakeRotator 0.0 (Variables|Stove|GetDial%2003%20Rotation) 0.0) false false)
  (Transformation|AddLocalRotation (Variables|Default|GetKitchen_Stove_05) (Math|Rotator|MakeRotator 0.0 (Variables|Stove|GetDial%2004%20Rotation) 0.0) false false)
  (Transformation|AddLocalRotation (Variables|Default|GetKitchen_Stove_09) (Math|Rotator|MakeRotator 0.0 (Variables|Stove|GetDial%2005%20Rotation) 0.0) false false)
  (bind _returnvalue (Rendering|Material|CreateDynamicMaterialInstance (Variables|Default|GetKitchen_Stove_03) 0 0 "" :!class /Script/Engine.PrimitiveComponent))
  (Rendering|Material|SetScalarParameterValue _returnvalue "Emissive Strength" (Variables|Stove|GetOven%20Emissive%20Strength) :!class /Script/Engine.MaterialInstanceDynamic)
  (Rendering|SetVisibility (Variables|Default|GetKitchen_Stove_04) (Variables|Stove|GetCable%20Visibile?) false))