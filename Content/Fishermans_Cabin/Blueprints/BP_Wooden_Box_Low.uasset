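; BP_Wooden_Box_Low is a low wooden box prop from the Fisherman's Cabin assets with a lid and two hooks that can be posed.
; The construction script adds local rotations to three mesh components: roll from LidAngle for the lid, and pitch from HookRightRotation and HookLeftRotation for the hooks.
; It has no runtime logic, as the event graph holds only disabled placeholder events.
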(event EventBeginPlay)

(event Collision|EventActorBeginOverlap
  (params (OtherActor :type Actor%20Object%20Reference)))

(event EventTick
  (params (DeltaSeconds :type Float%20%28single-precision%29)))

(fn ConstructionScript
  (Transformation|AddLocalRotation (Variables|Default|GetSM_Wooden_Box_Low_02) (Math|Rotator|MakeRotator (Variables|WoodenBoxLow|GetLid%20Angle) 0.0 0.0) false false)
  (Transformation|AddLocalRotation (Variables|Default|GetSM_Wooden_Box_Low_03) (Math|Rotator|MakeRotator 0.0 (Variables|WoodenBoxLow|GetHook%20Right%20Rotation) 0.0) false false)
  (Transformation|AddLocalRotation (Variables|Default|GetSM_Wooden_Box_Low_04) (Math|Rotator|MakeRotator 0.0 (Variables|WoodenBoxLow|GetHook%20Left%20Rotation) 0.0) false false))