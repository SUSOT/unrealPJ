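; BP_Candleplacer is a set-dressing actor for placing configurable candles, with all active logic in the Construction Script.
; Selector indices pick thin or thick candle meshes, optional wax spill meshes and matching flame meshes from arrays.
; An optional wax decal takes a set transform, and both candle and decal can get random rotation.
; Enabling the flame also sets emissive strength on the candle's materials.
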(event EventBeginPlay)

(event Collision|EventActorBeginOverlap
  (params (OtherActor :type Actor%20Object%20Reference)))

(event EventTick
  (params (DeltaSeconds :type Float%20%28single-precision%29)))

(fn ConstructionScript
  (bind _decal (Variables|Default|GetDecal))
  (bind _flame_emissive_strength (Variables|Default|GetFlame%20Emissive%20Strength))
  (if (Variables|Default|GetUse%20Thin%20Candles?)
    (Components|StaticMesh|SetStaticMesh (Variables|Default|GetCandle) (Utilities|Array|Get(acopy) (Variables|Default|GetThinCandlesArray) (Variables|Default|GetCandle%20Selector)))
    (else
      (Components|StaticMesh|SetStaticMesh (Variables|Default|GetCandle) (Utilities|Array|Get(acopy) (Variables|Default|GetThickCandlesArray) (Variables|Default|GetCandle%20Selector)))))
  (if (Variables|Default|GetUse%20Wax%20Spill?)
    (if (Variables|Default|GetUse%20Thin%20Candles?)
      (if (Variables|Default|GetUse%20Large%20Wax%20Spill%20for%20Thin%20Candle?)
        (Components|StaticMesh|SetStaticMesh (Variables|Default|GetWaxSpill) (Utilities|Array|Get(acopy) (Variables|Default|GetWaxSpillsThickArray) (Variables|Default|GetWax%20Spill%20Selector%20Thick)) :!label _label)
        (else
          (Components|StaticMesh|SetStaticMesh (Variables|Default|GetWaxSpill) (Utilities|Array|Get(acopy) (Variables|Default|GetWaxSpillsThinArray) (Variables|Default|GetWax%20Spill%20Selector%20Thin)))))
      (else
        (goto _label))))
  (if (Variables|Default|GetUse%20Wax%20Spill%20Decal?)
    (Transformation|SetRelativeTransform _decal (Variables|Default|GetDecal%20Transform) false false)
    (if (Variables|Default|GetAdd%20Random%20Rotation%20Decal?)
      (Transformation|SetRelativeRotation _decal (Math|Rotator|MakeRotator (Math|Random|RandomFloatinRange 0.0 3.6e+02) -9e+01 0.0) false false))
    (else
      (Rendering|SetVisibility _decal false false)))
  (if (Variables|Default|GetEnable%20Flame?)
    (if (Variables|Default|GetUse%20Thin%20Candles?)
      (Components|StaticMesh|SetStaticMesh (Variables|Default|GetFlame) (Utilities|Array|Get(acopy) (Variables|Default|GetCandleFlamesThin) (Variables|Default|GetCandle%20Selector)))
      (Rendering|Material|CreateDynamicMaterialInstance (Variables|Default|GetCandle) 0 0 "None" :!class /Script/Engine.PrimitiveComponent)
      (Rendering|Material|SetScalarParameterValueonMaterials (Variables|Default|GetCandle) "Emissive Strength" _flame_emissive_strength)
      (else
        (Components|StaticMesh|SetStaticMesh (Variables|Default|GetFlame) (Utilities|Array|Get(acopy) (Variables|Default|GetCandleFlamesThick) (Variables|Default|GetCandle%20Selector)))
        (Rendering|Material|CreateDynamicMaterialInstance (Variables|Default|GetCandle) 0 0 "None" :!class /Script/Engine.PrimitiveComponent)
        (Rendering|Material|SetScalarParameterValueonMaterials (Variables|Default|GetCandle) "Emissive Strength" _flame_emissive_strength))))
  (if (Variables|Default|GetAdd%20random%20rotation?)
    (Transformation|SetRelativeRotation (Variables|Default|GetCandle) (Math|Rotator|MakeRotator 0.0 0.0 (Math|Random|RandomFloatinRange 0.0 3.6e+02)) false false)))